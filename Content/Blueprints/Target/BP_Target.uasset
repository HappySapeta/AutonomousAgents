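; BP_Target is a target actor whose movement comes from a pluggable movement function object.
; On BeginPlay it constructs that object from the MovementFunctionType class and records its own starting location.
; Each Tick, while the object is valid, it asks it for an updated location using delta time and places the actor at that offset from the start, without sweeping.
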(event EventBeginPlay
  (bind _returnvalue (Game|ConstructObjectfromClass (Variables|Default|GetMovementFunctionType)))
  (Variables|Default|SetMovementFunction _returnvalue)
  (Variables|Default|SetStartingLocation (Transformation|GetActorLocation)))

(event EventTick
  (params (DeltaSeconds :type Float%20%28single-precision%29))
  (bind _movementfunction (Variables|Default|GetMovementFunction))
  (Utilities|IsValid _movementfunction
    (:Is%20Valid
      (bind _newlocation (Default|GetUpdatedLocation _movementfunction DeltaSeconds))
      (Transformation|SetActorLocation (+ _newlocation (Variables|Default|GetStartingLocation)) false false))))

(fn ConstructionScript)